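; Player controller for the Minesweeper game that routes movement, jump and menu input to the pawn and HUD.
; Move axes push the controlled pawn along fixed world directions rather than camera-relative ones, and Jump starts and stops jumping on MinesweeperCharacter_BP.
; ToggleNewGameMenu shows or hides the New Game menu through MinesweeperHUD_BP, only while neither the game-over nor win screen is visible.
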(event EventBeginPlay)

(event EventTick
  (params (DeltaSeconds :type Float%20%28single-precision%29)))

(event Input|ActionEvents|InputActionJump
  (params (Key :type Key%20Structure :default "None"))
  (bind _returnvalue (Pawn|GetControlledPawn))
  ;[1 1 1] Jumping
  (:Pressed
    (bind _asminesweeper_character_bp (Utilities|Casting|CastToMinesweeperCharacter_BP _returnvalue))
    (Character|Jump _asminesweeper_character_bp))
  (:Released
    (bind _asminesweeper_character_bp_2 (Utilities|Casting|CastToMinesweeperCharacter_BP _returnvalue))
    (Character|StopJumping _asminesweeper_character_bp_2)))

(event Input|ActionEvents|InputActionToggleNewGameMenu
  (params (Key :type Key%20Structure :default "None"))
  ;[1 1 1] New Game Menu
  (:Pressed
    (bind _asminesweeper_hud_bp (Utilities|Casting|CastToMinesweeperHUD_BP (HUD|GetHUD)))
    (if (Math|Boolean|NORBoolean (Variables|/Script/Minesweeper.MinesweeperHUDBase|GetbGameOverVisible _asminesweeper_hud_bp) (Variables|/Script/Minesweeper.MinesweeperHUDBase|GetbGameWinVisible _asminesweeper_hud_bp))
      (if (Variables|/Script/Minesweeper.MinesweeperHUDBase|GetbNewGameMenuVisible _asminesweeper_hud_bp)
        (Class|MinesweeperHUDBase|HideNewGameMenu _asminesweeper_hud_bp)
        (else
          (Class|MinesweeperHUDBase|ShowNewGameMenu _asminesweeper_hud_bp))))))

(event Input|AxisEvents|InputAxisMoveForward
  (params (AxisValue :type Float%20%28single-precision%29))
  (bind _returnvalue (Pawn|GetControlledPawn))
  ;[1 1 1] Movement input bindings
  (Utilities|IsValid _returnvalue
    (:Is%20Valid
      (Pawn|Input|AddMovementInput _returnvalue "0.000000,-90.000000, 0" AxisValue false))))

(event Input|AxisEvents|InputAxisMoveRight
  (params (AxisValue :type Float%20%28single-precision%29))
  (bind _returnvalue (Pawn|GetControlledPawn))
  ;[1 1 1] Movement input bindings
  (Utilities|IsValid _returnvalue
    (:Is%20Valid
      (Pawn|Input|AddMovementInput _returnvalue "90.000000,0.000000, 0" AxisValue false))))

(fn ConstructionScript)